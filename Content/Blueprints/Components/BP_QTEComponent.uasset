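; BP_QTEComponent runs a button-mashing quick time event for the player character.
; StartQTE disables movement, shows the W_QTEPB widget and starts a looping timer that drains Point, while CheckPressed adds points.
; CheckQTE calls fail at zero or success at 100, and ClearQTE restores walking, removes the widget and resets points.
; A slomo console-command helper exists but is only called disabled, and Tick prints Point for debugging.
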(event `self.ReceiveTick`
  (params (DeltaSeconds :type "Float (single-precision)"))
  (`KismetSystemLibrary.PrintString` (`KismetStringLibrary.Conv_IntToString` (`self.Point`)) true true (struct :`G` 0.66 :`B` 1.0 :`A` 1.0) 0.0))

(fn `CheckPressed`
  (bind _point (`self.Point`))
  (if (and (not (>= _point 100)) (`self.QTEStart`))
    (set `self.Point` (+ _point (`self.AddedPoint`)))))

(fn `CheckQTE`
  (bind _result (`/Engine/EditorBlueprintResources/StandardMacros.DecrementInt` (`self.Point`))
    (:`  `
      (bind _output_get (set `self.Point` _result))
      (if (<= _output_get 0)
        (`KismetSystemLibrary.PrintString` "Lose QTE" true true (struct :`R` 1.0 :`A` 1.0))
        (set `self.IsFail` true)
        (`self.ClearQTE`)
        (`self.QTEFail`)
        (elif (>= (`self.Point`) 100)
          (`KismetSystemLibrary.PrintString` "QTE win" true true (struct :`G` 1.0 :`A` 1.0))
          (set `self.IsSuccessfull` true)
          (`self.ClearQTE`)
          (`self.QTESuccessfull`))))))

(fn `ClearQTE`
  (`KismetSystemLibrary.K2_ClearAndInvalidateTimerHandle` (`self.CheckTimer`))
  (set `self.QTEStart` false)
  (`CharacterMovementComponent.SetMovementMode` (`self.GetCharacter`) "MOVE_Walking" 0)
  (`self.Slolmo` false)
  (`Widget.RemoveFromParent` (`self.QTEWidget`))
  (set `self.Point` (`self.DefaultQTEPoint`)))

(fn `GetCharacter`
  (returns (CharMove :type "CharacterMovementComponent Object Reference"))
  (return (`Character.CharacterMovement` (cast `/Game/Blueprints/Character/ThirdPersonCharacter` (`GameplayStatics.GetPlayerCharacter` 0) :!pure true))))

(fn `NewQTE`
  (params (QTEType :type "/Game/Data/Enums/E_QTEType Enum" :default "NewEnumerator0"))
  (switch `/Game/Data/Enums/E_QTEType` QTEType
    (:`NewEnumerator0`
      (bind _returnvalue (`KismetSystemLibrary.K2_SetTimer` null "CheckQTE" (`self.DerogationSpeed`) true))
      (set `self.CheckTimer` _returnvalue))))

(fn `Slolmo`
  (params (Enable :type Boolean))
  (if Enable
    (`KismetSystemLibrary.ExecuteConsoleCommand` "Slomo 0.7")
    (else
      (`KismetSystemLibrary.ExecuteConsoleCommand` "Slomo 1"))))

(fn `StartQTE`
  (`self.NewQTE` "NewEnumerator0")
  (set `self.QTEStart` true)
  (`CharacterMovementComponent.DisableMovement` (`self.GetCharacter`))
  (`self.Slolmo` false)
  (bind _returnvalue (`|CreateWidget` "/Game/UI/QTEProgressBar/W_QTEPB.W_QTEPB_C" (`GameplayStatics.GetPlayerController` 0)))
  (bind _output_get (set `self.QTEWidget` _returnvalue))
  (`UserWidget.AddToViewport` _output_get 0))